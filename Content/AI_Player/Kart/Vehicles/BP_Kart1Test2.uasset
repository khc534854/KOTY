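; Test kart Blueprint that drives itself along a road spline, with no input or physics in its own graph.
; On BeginPlay it finds a BP_SplineRoad actor and starts the MoveObjectT timeline, with play rate set from TimeToCompleteInSeconds.
; Each update maps the timeline alpha to distance along RoadSpline and sets the actor transform.
; Location is sampled in world space but rotation in spline-local space.
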(event `self.ReceiveBeginPlay`
  (`parent.ReceiveBeginPlay`)
  (bind _returnvalue (`GameplayStatics.GetActorOfClass` "/Game/AI_Player/TestLevel/BP_SplineRoad.BP_SplineRoad_C"))
  (set `self.Spline REF1` _returnvalue)
  (`self.Move Object`))

(event `Move Object`
  (bind _roadspline (`/Game/AI_Player/TestLevel/BP_SplineRoad.RoadSpline` (`self.Spline REF1`)))
  (`TimelineComponent.SetPlayRate` (`self.Move Object T`) (/ 1.0 (`self.TimeToComplete(In seconds)`)))
  (bind (_direction _movetrack) (`Timeline|Move Object T`)
    (:`Update`
      (bind _returnvalue (`KismetMathLibrary.Lerp` 0.0 (`SplineComponent.GetSplineLength` (`/Game/AI_Player/TestLevel/BP_SplineRoad.RoadSpline` (`self.Spline REF1`))) _movetrack))
      (`self.K2_SetActorTransform` (`KismetMathLibrary.MakeTransform` (`SplineComponent.GetLocationAtDistanceAlongSpline` _roadspline _returnvalue "World") (`SplineComponent.GetRotationAtDistanceAlongSpline` _roadspline _returnvalue "Local"))))))

(fn `UserConstructionScript`
  (`parent.UserConstructionScript`))