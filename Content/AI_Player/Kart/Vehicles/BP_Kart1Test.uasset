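; BP_Kart1Test is a test kart that moves along a road spline.
; BeginPlay caches the first BP_SplineRoadTest found in the level.
; The MoveObject event plays a timeline, rate-scaled by TimeToCompleteInSeconds, lerping distance from zero to the spline's length and setting the actor's transform each update.
; Location is sampled in world space but rotation in local space, and nothing here calls MoveObject.
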(event `self.ReceiveBeginPlay`
  (`parent.ReceiveBeginPlay`)
  (bind _returnvalue (`GameplayStatics.GetActorOfClass` "/Game/AI_Player/TestLevel/BP_SplineRoadTest.BP_SplineRoadTest_C"))
  (set `self.Spline REF` _returnvalue))

(event `Move Object`
  (bind _spline (`/Game/AI_Player/TestLevel/BP_SplineRoadTest.Spline` (`self.Spline REF`)))
  (`TimelineComponent.SetPlayRate` (`self.Move Object T`) (/ 1.0 (`self.TimeToComplete(In seconds)`)))
  (bind (_direction _movetrack) (`Timeline|Move Object T`)
    (:`Update`
      (bind _returnvalue (`KismetMathLibrary.Lerp` 0.0 (`SplineComponent.GetSplineLength` (`/Game/AI_Player/TestLevel/BP_SplineRoadTest.Spline` (`self.Spline REF`))) _movetrack))
      (`self.K2_SetActorTransform` (`KismetMathLibrary.MakeTransform` (`SplineComponent.GetLocationAtDistanceAlongSpline` _spline _returnvalue "World") (`SplineComponent.GetRotationAtDistanceAlongSpline` _spline _returnvalue "Local"))))))

(fn `UserConstructionScript`
  (`parent.UserConstructionScript`))