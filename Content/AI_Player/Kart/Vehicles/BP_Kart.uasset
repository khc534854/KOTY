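; BP_Kart is a drivable physics kart that fakes suspension and drive with forces on a Box body.
; Each tick, four wheel traces apply distance-scaled spring forces and move the wheel meshes.
; Grounded wheels also apply forward drive and shift the center of mass with throttle.
; Enhanced Input smooths throttle, which decays each tick and scales steering torque; a derived Acceleration value spins the wheel meshes.
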(event `EnhancedInput|/Game/AI_Player/Kart/Input/IA_Accelerate`
  (params (ActionValue :type "Float (double-precision)") (ElapsedSeconds :type "Float (double-precision)") (TriggeredSeconds :type "Float (double-precision)") (InputAction :type "InputAction Object Reference" :default "/Game/AI_Player/Kart/Input/IA_Accelerate.IA_Accelerate"))
  (bind _returnvalue (`KismetMathLibrary.FInterpTo` (`self.AccelerationInput`) ActionValue (`GameplayStatics.GetWorldDeltaSeconds`) 1.0))
  (:`Triggered`
    (set `self.AccelerationInput` _returnvalue)
    (`KismetSystemLibrary.PrintString` (`KismetStringLibrary.Conv_DoubleToString` _returnvalue))))

(event `self.ReceiveBeginPlay`
  ; begin 시 IMC_Vehicle context추가
  (`EnhancedInputSubsystemInterface.AddMappingContext` (pcsubsystem `EnhancedInputLocalPlayerSubsystem` (`GameplayStatics.GetPlayerController` 0)) "/Game/AI_Player/Kart/Input/IMC_Vehicle.IMC_Vehicle" 0 (struct)))

(event `EnhancedInput|/Game/AI_Player/Kart/Input/IA_Steer`
  (params (ActionValue :type "Float (double-precision)") (ElapsedSeconds :type "Float (double-precision)") (TriggeredSeconds :type "Float (double-precision)") (InputAction :type "InputAction Object Reference" :default "/Game/AI_Player/Kart/Input/IA_Steer.IA_Steer"))
  (:`Triggered`
    (`PrimitiveComponent.AddTorqueInRadians` (`self.Box`) (`KismetMathLibrary.MakeVector` 0.0 0.0 (* ActionValue 10000000.0 (`self.AccelerationInput`))) "None" false)))

(event `self.ReceiveTick`
  (params (DeltaSeconds :type "Float (single-precision)"))
  (`self.SuspensionCast` (`self.BR_Wheel`))
  (`self.SuspensionCast` (`self.BL_Wheel`))
  (`self.SuspensionCast` (`self.FL_Wheel`))
  (`self.SuspensionCast` (`self.FR_Wheel`))
  (`self.CalculateAcceleration`))

(fn `AccelerateKart`
  (params (Wheel :type "SceneComponent Object Reference"))
  (bind _box (`self.Box`))
  (`PrimitiveComponent.AddForceAtLocation` (`self.Box`) (* (`SceneComponent.GetForwardVector` _box) 1000.0 (`self.AccelerationInput`) (`PrimitiveComponent.GetMass` _box)) (`SceneComponent.K2_GetComponentLocation` Wheel) "None")
  (`PrimitiveComponent.SetCenterOfMass` (`self.Box`) (* (50.0 0.0 0.0) (`self.AccelerationInput`)) "None"))

(fn `CalculateAcceleration`
  (bind _accelerationinput (`self.AccelerationInput`))
  ; Acceleration은 항상 양수만 나온다. 방향은 따로 곱해준다
  (bind _output_get (set `self.Acceleration` (* (`KismetMathLibrary.Lerp` 0.0 15000.0 _accelerationinput) _accelerationinput)))
  ; w키,s키를 누르지 않고 있으면 Acceleration Input을
  ; 0으로 수렴시킨다.
  (set `self.AccelerationInput` (`KismetMathLibrary.FInterpTo` (`self.AccelerationInput`) 0.0 (`GameplayStatics.GetWorldDeltaSeconds`) 0.3))
  (`SceneComponent.K2_AddLocalRotation` (`self.WheelMesh_FR`) (`KismetMathLibrary.MakeRotator` 0.0 (/ _output_get -1000.0)) false false)
  (`SceneComponent.K2_AddLocalRotation` (`self.WheelMesh_FL`) (`KismetMathLibrary.MakeRotator` 0.0 (/ _output_get -1000.0)) false false)
  (`SceneComponent.K2_AddLocalRotation` (`self.WheelMesh_BL`) (`KismetMathLibrary.MakeRotator` 0.0 (/ _output_get -1000.0)) false false)
  (`SceneComponent.K2_AddLocalRotation` (`self.WheelMesh_BR`) (`KismetMathLibrary.MakeRotator` 0.0 (/ _output_get -1000.0)) false false))

(fn `SuspensionCast`
  (params (WheelComp :type "SceneComponent Object Reference"))
  (bind _returnvalue (`SceneComponent.K2_GetComponentLocation` WheelComp))
  (bind _returnvalue_2 (`SceneComponent.GetChildComponent` (`local.WheelComp`) 0))
  (bind (_relativelocation_x _relativelocation_y _relativelocation_z) (`KismetMathLibrary.BreakVector` (`SceneComponent.RelativeLocation` _returnvalue_2)))
  ; suspension의 위치를 가져와서 차에서 아래로 -60만큼 trace를 쏨
  (bind _outhit (`KismetSystemLibrary.LineTraceSingle` :`Start` _returnvalue :`End` (+ _returnvalue (* (`SceneComponent.GetUpVector` WheelComp) -60.0)) :`TraceChannel` "TraceTypeQuery1" :`DrawDebugType` "ForDuration"))
  (bind (_bblockinghit _binitialoverlap _time _distance _location _impactpoint _normal _impactnormal _physmat _hitactor _hitcomponent _hitbonename _bonename _hititem _elementindex _faceindex _tracestart _traceend) (`GameplayStatics.BreakHitResult` _outhit))
  (if _bblockinghit
    ; WheelComp가 있는 위치에 들어올려지는 힘을 줌
    (`PrimitiveComponent.AddForceAtLocation` (`self.Box`) (* (* (- 1.0 (`KismetMathLibrary.NormalizeToRange` _distance 0.0 60.0)) (`KismetMathLibrary.GetDirectionUnitVector` _traceend _tracestart)) (`self.SuspensionPower`)) (`SceneComponent.K2_GetComponentLocation` (`local.WheelComp`)) "None")
    (`self.AccelerateKart` (`local.WheelComp`))
    (`SceneComponent.K2_SetRelativeLocation` _returnvalue_2 (`KismetMathLibrary.MakeVector` 0.0 0.0 (`KismetMathLibrary.FInterpTo` _relativelocation_z (+ (* _distance -1.0) 32.0) (`GameplayStatics.GetWorldDeltaSeconds`) 3.0)) false false)))

(fn `UserConstructionScript`)