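; AI test kart that follows a BP_SplineRoad1 spline and triggers its held item on a looping timer.
; BeginPlay picks the road via FindNearestSpline, whose reversed loop and zero starting distance always yield the first actor found.
; Tick aims at a speed-scaled look-ahead point, mapping yaw error to steering and target speed for throttle or braking.
; Steering is computed only when DebugSteering is true; its debug drawing is disconnected.
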(event `CustomEvent`
  (`KotyItemHoldComponent.UseCurrentItem` (`self.KotyItemHold`)))

(event `self.ReceiveBeginPlay`
  (bind _boxcomponent (`self.BoxComponent`))
  (bind _outactors (`GameplayStatics.GetAllActorsOfClass` "/Game/AI_Player/TestLevel/BP_SplineRoad1.BP_SplineRoad1_C"))
  (bind _splineactor (`self.FindNearestSpline` _outactors))
  (set `self.DefaultSpline` _splineactor)
  (set `self.SplineActor` (`self.DefaultSpline`))
  (set `self.DefaultMaxSpeed` (`self.MaxSpeed`))
  (`KismetSystemLibrary.ExecuteConsoleCommand` "ShowFlag.Splines 1" null)
  (`KismetSystemLibrary.K2_SetTimerDelegate` (delegate `CustomEvent`) 5.0 true)
  (`SceneComponent.K2_AttachToComponent` (`self.KotyItemHold`) _boxcomponent "None" "KeepRelative" "KeepRelative" "KeepRelative" true)
  (`SceneComponent.K2_AttachToComponent` (`self.KotyItemHit`) _boxcomponent "None" "KeepRelative" "KeepRelative" "KeepRelative" true))

(event `self.ReceiveTick`
  (params (DeltaSeconds :type "Float (single-precision)"))
  (`/Engine/EditorBlueprintResources/StandardMacros.IsValid` (`self.SplineActor`)
    (:`Is Valid`
      (`|ExecutionSequence`
        (:`then_0`
          (bind _returnvalue (`self.CalculateSteeringInput` (`self.SplineActor`)))
          (set `self.HandlingDir` _returnvalue))
        (:`then_1`
          (set `self.TargetSpeed` (`KismetMathLibrary.MapRangeClamped` (`KismetMathLibrary.Abs` (`self.YawDelta`)) 30.0 5.0 (`self.MinSpeed`) (`self.MaxSpeed`)))
          (if (< (`self.CurSpeed`) (`self.TargetSpeed`))
            (set `self.AccelerationDir` 1.0)
            (else
              (set `self.AccelerationDir` -1.0))))))))

(fn `CalculateSteeringInput`
  (params (Spline :type "/Game/AI_Player/TestLevel/BP_SplineRoad1 Object Reference"))
  (returns (ReturnValue :type "Float (double-precision)"))
  (locals (OffsetTangentLocation :type "Vector Structure") (DebugSteering :type Boolean :default true))
  (bind _returnvalue (`self.K2_GetActorLocation`))
  (bind _roadspline (`/Game/AI_Player/TestLevel/BP_SplineRoad1.RoadSpline` Spline))
  (bind _returnvalue_2 (`SplineComponent.FindLocationClosestToWorldLocation` _roadspline (+ _returnvalue (* (`KismetMathLibrary.Normal` (`SplineComponent.FindTangentClosestToWorldLocation` _roadspline _returnvalue "World")) (`self.CurSpeed`))) "World"))
  (bind (_returnvalue_roll _returnvalue_pitch _returnvalue_yaw) (`KismetMathLibrary.BreakRotator` (`KismetMathLibrary.NormalizedDeltaRotator` (`KismetMathLibrary.FindLookAtRotation` (`self.K2_GetActorLocation`) _returnvalue_2) (`self.K2_GetActorRotation`))))
  (bind _output_get (set `local.OffsetTangentLocation` _returnvalue_2))
  (if (`local.DebugSteering`)
    (set `self.YawDelta` _returnvalue_yaw)
    (return (`KismetMathLibrary.MapRangeClamped` _returnvalue_yaw -30.0 30.0 -1.0 1.0))))

(fn `FindNearestSpline`
  (params (SplineActors :type "Array of /Game/AI_Player/TestLevel/BP_SplineRoad1 Object Reference"))
  (returns (SplineActor :type "/Game/AI_Player/TestLevel/BP_SplineRoad1 Object Reference"))
  (locals (Distance :type "Float (double-precision)") (NearestSpline :type "/Game/AI_Player/TestLevel/BP_SplineRoad1 Object Reference"))
  (bind _returnvalue (`self.K2_GetActorLocation`))
  (set `local.Distance` 0.0)
  (bind (_arrayindex _arrayelement) (`/Engine/EditorBlueprintResources/StandardMacros.ReverseForEachLoop` SplineActors)
    (:`LoopBody`
      (if (== _arrayindex 0)
        (bind _returnvalue_2 (`KismetMathLibrary.Vector_Distance` (`SplineComponent.FindLocationClosestToWorldLocation` (`/Game/AI_Player/TestLevel/BP_SplineRoad1.RoadSpline` _arrayelement) _returnvalue "Local") _returnvalue))
        (set `local.Distance` _returnvalue_2 :!label _label)
        (set `local.NearestSpline` _arrayelement)
        (elif (< _returnvalue_2 (`local.Distance`))
          (goto _label))))
    (:`Completed`
      (return (`local.NearestSpline`)))))

(fn `UserConstructionScript`)