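; BP_KartAI is an AI kart Blueprint meant to follow the road splines placed in the level.
; On BeginPlay it picks the nearest BP_SplineRoad as its default and active spline, measuring closest spline points in local space against its world location, and caches MaxSpeed.
; Tick passes the active spline to CalculateSteeringInput, which is an empty stub with only unconnected tangent math.
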(event `self.ReceiveBeginPlay`
  (`parent.ReceiveBeginPlay`)
  (bind _outactors (`GameplayStatics.GetAllActorsOfClass` "/Game/AI_Player/TestLevel/BP_SplineRoad.BP_SplineRoad_C"))
  (bind _splineactor (`self.FindNearestSpline` _outactors))
  (set `self.DefaultSpline` _splineactor)
  (set `self.SplineActor` (`self.DefaultSpline`))
  (set `self.DefaultMaxSpeed` (`self.MaxSpeed`)))

(event `self.ReceiveTick`
  (params (DeltaSeconds :type "Float (single-precision)"))
  (`parent.ReceiveTick` DeltaSeconds)
  (`/Engine/EditorBlueprintResources/StandardMacros.IsValid` (`self.SplineActor`)
    (:`Is Valid`
      (`|ExecutionSequence`
        (:`then_0`
          (`self.CalculateSteeringInput` (`self.SplineActor`)))))))

(fn `CalculateSteeringInput`
  (params (Spline :type "/Game/AI_Player/TestLevel/BP_SplineRoad Object Reference")))

(fn `FindNearestSpline`
  (params (SplineActors :type "Array of /Game/AI_Player/TestLevel/BP_SplineRoad Object Reference"))
  (returns (SplineActor :type "/Game/AI_Player/TestLevel/BP_SplineRoad Object Reference"))
  (locals (Distance :type "Float (double-precision)") (NearestSpline :type "/Game/AI_Player/TestLevel/BP_SplineRoad Object Reference"))
  (bind _returnvalue (`self.K2_GetActorLocation`))
  (set `local.Distance` 0.0)
  (for (_array_element _array_index) SplineActors
    (if (== _array_index 0)
      (bind _returnvalue_2 (`KismetMathLibrary.Vector_Distance` (`SplineComponent.FindLocationClosestToWorldLocation` (`/Game/AI_Player/TestLevel/BP_SplineRoad.RoadSpline` _array_element) _returnvalue "Local") _returnvalue))
      (set `local.Distance` _returnvalue_2 :!label _label)
      (set `local.NearestSpline` _array_element)
      (elif (< _returnvalue_2 (`local.Distance`))
        (goto _label))))
  (return (`local.NearestSpline`)))

(fn `UserConstructionScript`
  (`parent.UserConstructionScript`))