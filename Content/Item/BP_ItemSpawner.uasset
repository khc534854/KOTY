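; Item spawner actor that launches green turtle, red turtle and black bomb items from its Arrow component.
; Each throw event spawns the item and starts its MoveComp simulation: constant horizontal speed for turtles, linear drag for bombs.
; Throwing also sets a ten-second lifespan on the spawner itself, not the item.
; When Rotate is set, Tick sweeps the Arrow's yaw sinusoidally at a fixed upward pitch.
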(event `ThrowTurtle`
  ; Comment
  (bind _returnvalue (`|SpawnActorFromClass` "/Game/Item/BP_GreenTurtleItemFinal.BP_GreenTurtleItemFinal_C" (`SceneComponent.K2_GetComponentToWorld` (`self.Arrow`)) "Undefined" "MultiplyWithRoot" null null))
  (`KotyMovementComponent.ThrowConstantHorizon` (`PhysicItemBase.MoveComp` _returnvalue) true (0.0 0.0 -1.0) 9000.0 3000.0 4.0 (* (`SceneComponent.GetForwardVector` (`self.Arrow`)) 3000.0) 0.25)
  (`self.SetLifeSpan` 10.0))

(event `ThrowBomb`
  ; Comment
  (bind _returnvalue (`|SpawnActorFromClass` "/Game/Item/BlackBomb/BP_BlackBombItemFinal.BP_BlackBombItemFinal_C" (`SceneComponent.K2_GetComponentToWorld` (`self.Arrow`)) "Undefined" "MultiplyWithRoot" null null))
  (`KotyMovementComponent.ThrowLinearDrag` (`PhysicItemBase.MoveComp` _returnvalue) true (0.0 0.0 -1.0) 6000.0 5.0 4.0 (* (`SceneComponent.GetForwardVector` (`self.Arrow`)) 4500.0) 0.25)
  (`self.SetLifeSpan` 10.0))

(event `ThrowRedTurtle`
  ; Comment
  (bind _returnvalue (`|SpawnActorFromClass` "/Game/Item/BP_RedTurtleItemFinal.BP_RedTurtleItemFinal_C" (`SceneComponent.K2_GetComponentToWorld` (`self.Arrow`)) "Undefined" "MultiplyWithRoot" null null))
  (`KotyMovementComponent.ThrowConstantHorizon` (`PhysicItemBase.MoveComp` _returnvalue) true (0.0 0.0 -1.0) 9000.0 3000.0 4.0 (* (`SceneComponent.GetForwardVector` (`self.Arrow`)) 3000.0) 0.25)
  (`self.SetLifeSpan` 10.0))

(event `self.ReceiveTick`
  (params (DeltaSeconds :type "Float (single-precision)"))
  (if (`self.Rotate?`)
    (bind _output_get (set `self.ElapsedTime` (+ DeltaSeconds (`self.ElapsedTime`))))
    (`SceneComponent.K2_SetWorldRotation` (`self.Arrow`) (`KismetMathLibrary.MakeRotator` 0.0 45.0 (* (`KismetMathLibrary.Sin` _output_get) 45.0)) false false)))

(fn `UserConstructionScript`)