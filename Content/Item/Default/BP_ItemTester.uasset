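; BP_ItemTester is a debug actor that triggers item throws from keyboard input for testing.
; On BeginPlay it gathers every BP_PhysicsItemTester in the level into ThrowItemTesters.
; The J, K and L keys loop over that list and tell each active tester to throw a bomb, turtle or red turtle respectively.
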(event `self.ReceiveBeginPlay`
  (bind _outactors (`GameplayStatics.GetAllActorsOfClass` "/Game/Item/PhysicsItem/BP_PhysicsItemTester.BP_PhysicsItemTester_C"))
  (set `self.ThrowItemTesters` _outactors))

(event `Key|K`
  (params (Key :type "Key Structure"))
  (:`Pressed`
    (for _array_element (`self.ThrowItemTesters`)
      (if (`/Game/Item/PhysicsItem/BP_PhysicsItemTester.Active?` _array_element)
        (`/Game/Item/PhysicsItem/BP_PhysicsItemTester.ThrowTurtle` _array_element)))))

(event `Key|J`
  (params (Key :type "Key Structure"))
  (:`Pressed`
    (for _array_element (`self.ThrowItemTesters`)
      (if (`/Game/Item/PhysicsItem/BP_PhysicsItemTester.Active?` _array_element)
        (`/Game/Item/PhysicsItem/BP_PhysicsItemTester.ThrowBomb` _array_element)))))

(event `Key|L`
  (params (Key :type "Key Structure"))
  (:`Pressed`
    (for _array_element (`self.ThrowItemTesters`)
      (if (`/Game/Item/PhysicsItem/BP_PhysicsItemTester.Active?` _array_element)
        (`/Game/Item/PhysicsItem/BP_PhysicsItemTester.ThrowRedTurtle` _array_element)))))

(fn `UserConstructionScript`)