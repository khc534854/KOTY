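; BP_RoadSpline is a road actor that builds a deformed mesh along its Road spline.
; The construction script adds a spline mesh component per segment, copying local locations and tangents from both bounding points and setting only the end roll from the next point's rotation.
; Each piece attaches to the root with BlockAll query and physics collision.
; BeginPlay prints every point's local tangent as debug output.
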(event `self.ReceiveBeginPlay`
  (for _index (range (`SplineComponent.GetNumberOfSplinePoints` (`self.Road`)))
    (`KismetSystemLibrary.PrintString` (`KismetStringLibrary.Conv_VectorToString` (`SplineComponent.GetTangentAtSplinePoint` (`self.Road`) _index "Local")) true true (struct :`G` 0.66 :`B` 1.0 :`A` 1.0) 100.0)))

(fn `UserConstructionScript`
  (locals (LocalSplineMeshComp :type "SplineMeshComponent Object Reference"))
  (bind _localsplinemeshcomp (`local.LocalSplineMeshComp`))
  (for _index (range (+ (- (`SplineComponent.GetNumberOfSplinePoints` (`self.Road`)) 2) 1))
    (bind _returnvalue (`AddComponent|NODE_AddSplineMeshComponent-0`))
    (set `local.LocalSplineMeshComp` _returnvalue)
    (`|ExecutionSequence`
      (:`then_0`
        (bind (_location _tangent) (`SplineComponent.GetLocationAndTangentAtSplinePoint` (`self.Road`) _index "Local"))
        (bind (_location_2 _tangent_2) (`SplineComponent.GetLocationAndTangentAtSplinePoint` (`self.Road`) (+ _index 1) "Local"))
        ; Comment
        (`SplineMeshComponent.SetStartAndEnd` (`local.LocalSplineMeshComp`) _location _tangent _location_2 _tangent_2 true))
      (:`then_1`
        (bind _returnvalue_roll (`KismetMathLibrary.BreakRotator` (`SplineComponent.GetRotationAtSplinePoint` (`self.Road`) (+ _index 1) "Local")))
        (`SplineMeshComponent.SetEndRollDegrees` (`local.LocalSplineMeshComp`) _returnvalue_roll true))
      (:`then_2`
        ; Comment
        (`SceneComponent.K2_AttachToComponent` _localsplinemeshcomp (`self.DefaultSceneRoot`) "None" "KeepRelative" "KeepWorld" "KeepRelative" true)
        (`PrimitiveComponent.SetCollisionEnabled` _localsplinemeshcomp "QueryAndPhysics")
        (`PrimitiveComponent.SetCollisionProfileName` _localsplinemeshcomp "BlockAll" true)))))