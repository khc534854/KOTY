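; Throwable black bomb item that explodes on a five-second fuse, or immediately when it begins overlapping another physics item.
; Throw launches it along the given direction through KotyMovement's linear-drag simulation with strong downward gravity.
; Explosion currently only runs a debug-drawn sphere trace at the bomb's location and destroys the actor; the trace result is unused, so no damage is applied.
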(event `self.ReceiveBeginPlay`
  (bind _returnvalue (`KismetSystemLibrary.K2_SetTimerDelegate` (delegate `Explode`) 5.0))
  (set `self.ExplosionTimer` _returnvalue))

(event `Explode`
  (bind _returnvalue (`self.K2_GetActorLocation`))
  (`KismetSystemLibrary.SphereTraceSingle` :`Start` _returnvalue :`End` _returnvalue :`Radius` 800.0 :`TraceChannel` "TraceTypeQuery1" :`DrawDebugType` "ForDuration")
  (`self.K2_DestroyActor`))

(event `self.ReceiveActorBeginOverlap`
  (params (OtherActor :type "Actor Object Reference"))
  (cast `/Game/Item/PhysicsItem/BP_PhysicsItemBase` OtherActor)
  (`KismetSystemLibrary.K2_ClearAndInvalidateTimerHandle` (`self.ExplosionTimer`))
  (`self.Explode`))

(fn `Throw`
  (params (InMoveDir :type "Vector Structure"))
  (`KotyMovementComponent.ThrowLinearDrag` (`self.KotyMovement`) true (`KismetMathLibrary.Vector_Down`) 6000.0 5.0 3.0 (* InMoveDir 4500.0) 0.0))

(fn `UserConstructionScript`
  (`parent.UserConstructionScript`))