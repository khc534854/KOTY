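; BP_PhysicsItemTester is a test actor that launches physics items: green turtle, red turtle and black bomb.
; Each throw event spawns its item at the Arrow transform, calls Throw from BP_PhysicsItemBase along the arrow's forward vector, and gives it a short lifespan.
; When Rotate is set, Tick swings the arrow's yaw back and forth on a sine wave at a fixed pitch, varying the throw direction.
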(event `ThrowTurtle`
  ; Comment
  (bind _returnvalue (`|SpawnActorFromClass` "/Game/Item/PhysicsItem/BP_GreenTurtleItem.BP_GreenTurtleItem_C" (`SceneComponent.K2_GetComponentToWorld` (`self.Arrow`)) "Undefined" "MultiplyWithRoot" null null))
  (bind _asbp_physics_item_base (cast `/Game/Item/PhysicsItem/BP_PhysicsItemBase` _returnvalue))
  (`/Game/Item/PhysicsItem/BP_PhysicsItemBase.Throw` _asbp_physics_item_base (`SceneComponent.GetForwardVector` (`self.Arrow`)))
  (`self.SetLifeSpan` _asbp_physics_item_base 10.0))

(event `ThrowBomb`
  ; Comment
  (bind _returnvalue (`|SpawnActorFromClass` "/Game/Item/PhysicsItem/BP_BlackBombItem.BP_BlackBombItem_C" (`SceneComponent.K2_GetComponentToWorld` (`self.Arrow`)) "Undefined" "MultiplyWithRoot" null null))
  (bind _asbp_physics_item_base (cast `/Game/Item/PhysicsItem/BP_PhysicsItemBase` _returnvalue))
  (`/Game/Item/PhysicsItem/BP_PhysicsItemBase.Throw` _asbp_physics_item_base (`SceneComponent.GetForwardVector` (`self.Arrow`)))
  (`self.SetLifeSpan` _asbp_physics_item_base 10.0))

(event `ThrowRedTurtle`
  ; Comment
  (bind _returnvalue (`|SpawnActorFromClass` "/Game/Item/TrackingItem/BP_RedTurtle.BP_RedTurtle_C" (`SceneComponent.K2_GetComponentToWorld` (`self.Arrow`)) "Undefined" "MultiplyWithRoot" null null))
  (bind _asbp_physics_item_base (cast `/Game/Item/PhysicsItem/BP_PhysicsItemBase` _returnvalue))
  (`/Game/Item/PhysicsItem/BP_PhysicsItemBase.Throw` _asbp_physics_item_base (`SceneComponent.GetForwardVector` (`self.Arrow`)))
  (`self.SetLifeSpan` _asbp_physics_item_base 10.0))

(event `self.ReceiveTick`
  (params (DeltaSeconds :type "Float (single-precision)"))
  (if (`self.Rotate?`)
    (bind _output_get (set `self.ElapsedTime` (+ DeltaSeconds (`self.ElapsedTime`))))
    (`SceneComponent.K2_SetWorldRotation` (`self.Arrow`) (`KismetMathLibrary.MakeRotator` 0.0 45.0 (* (`KismetMathLibrary.Sin` _output_get) 45.0)) false false)))

(fn `UserConstructionScript`)