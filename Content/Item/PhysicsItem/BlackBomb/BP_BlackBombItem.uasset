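; A throwable black bomb item that explodes after a five-second fuse, or immediately when it overlaps another physics item.
; A timeline feeds elapsed time into a dynamic material on the sphere mesh to animate it during the countdown.
; Exploding spawns a BP_ExplosionTracer at the bomb's transform and destroys the bomb.
; Throw launches it along the given direction through KotyMovement's linear-drag simulation with heavy downward gravity.
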(event `self.ReceiveBeginPlay`
  ; 폭발 타이머
  (bind _returnvalue (`KismetSystemLibrary.K2_SetTimerDelegate` (delegate `Explode`) 5.0))
  (set `self.ExplosionTimer` _returnvalue)
  ; 폭탄병 머터리얼 인스턴스 패러미터
  (bind _returnvalue_2 (`PrimitiveComponent.CreateDynamicMaterialInstance` (`self.SphereMesh`) 0 "/Game/Item/PhysicsItem/BlackBomb/MT_BlackBomb.MT_BlackBomb" "None"))
  (bind _output_get (set `self.MeshMaterial` _returnvalue_2))
  (bind (_direction _elapsedtime) (`Timeline|Timeline`)
    (:`Update`
      (`MaterialInstanceDynamic.SetScalarParameterValue` _output_get "ElapsedTime" _elapsedtime))))

(event `Explode`
  ; 폭발 타이머
  (`|SpawnActorFromClass` "/Game/Item/PhysicsItem/BlackBomb/BP_ExplosionTracer.BP_ExplosionTracer_C" (`self.GetTransform`) "Undefined" "MultiplyWithRoot" null null)
  (`self.K2_DestroyActor`))

(event `self.ReceiveActorBeginOverlap`
  (params (OtherActor :type "Actor Object Reference"))
  ; 기타 대상과 충돌할 경우 폭발
  (cast `/Game/Item/PhysicsItem/BP_PhysicsItemBase` OtherActor)
  (`KismetSystemLibrary.K2_ClearAndInvalidateTimerHandle` (`self.ExplosionTimer`))
  (`self.Explode`))

(fn `Throw`
  (params (InMoveDir :type "Vector Structure"))
  (`KotyMovementComponent.ThrowLinearDrag` (`self.KotyMovement`) true (`KismetMathLibrary.Vector_Down`) 6000.0 5.0 3.0 (* InMoveDir 4500.0) 0.0))

(fn `UserConstructionScript`
  (`parent.UserConstructionScript`))