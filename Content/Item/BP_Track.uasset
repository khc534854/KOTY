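; BP_Track is a spline-driven track actor that builds a solid, deformed mesh along its spline in the Construction Script.
; It adds one SplineMeshComponent per segment, copying local positions, tangents and the start point's up vector from the spline.
; Roll accumulates by a fixed step (NewVar) per segment, so the track twists continuously along its length.
; Each piece attaches to the root with BlockAll collision; the event graph is unused.
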(fn `UserConstructionScript`
  (locals (Index :type Integer) (SplineMeshComp :type "SplineMeshComponent Object Reference"))
  (bind _spline (`self.Spline`))
  (bind (_location _tangent) (`SplineComponent.GetLocationAndTangentAtSplinePoint` _spline (`local.Index`) "Local"))
  (bind _returnvalue (* (`self.NewVar`) (`local.Index`)))
  (bind (_location_2 _tangent_2) (`SplineComponent.GetLocationAndTangentAtSplinePoint` _spline (+ (`local.Index`) 1) "Local"))
  (for _index (range (+ (- (`SplineComponent.GetNumberOfSplinePoints` (`self.Spline`)) 2) 1))
    (set `local.Index` _index)
    (bind _returnvalue_2 (`AddComponent|NODE_AddSplineMeshComponent-0`))
    (set `local.SplineMeshComp` _returnvalue_2)
    (`SplineMeshComponent.SetStartAndEnd` (`local.SplineMeshComp`) _location _tangent _location_2 _tangent_2 true)
    (`SplineMeshComponent.SetStartRollDegrees` (`local.SplineMeshComp`) _returnvalue true)
    (`SplineMeshComponent.SetEndRollDegrees` (`local.SplineMeshComp`) (+ _returnvalue (`self.NewVar`)) true)
    (`SplineMeshComponent.SetSplineUpDir` (`local.SplineMeshComp`) (`SplineComponent.GetUpVectorAtSplinePoint` (`self.Spline`) (`local.Index`) "Local") true)
    ; Comment
    (`SceneComponent.K2_AttachToComponent` (`local.SplineMeshComp`) (`self.DefaultSceneRoot`) "None" "KeepRelative" "KeepWorld" "KeepRelative" true)
    (`PrimitiveComponent.SetCollisionEnabled` (`local.SplineMeshComp`) "QueryAndPhysics")
    (`PrimitiveComponent.SetCollisionProfileName` (`local.SplineMeshComp`) "BlockAll" true)))