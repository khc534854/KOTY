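; BP_ItemTester is a test Blueprint that triggers item throws from keyboard input.
; On BeginPlay it collects every BP_ThrowItemTester in the level into an array.
; Pressing K calls ThrowTurtle and pressing J calls ThrowBomb on each tester in that array whose Active flag is set.
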(event `self.ReceiveBeginPlay`
  (bind _outactors (`GameplayStatics.GetAllActorsOfClass` "/Game/Item/ThrowItem/BP_ThrowItemTester.BP_ThrowItemTester_C"))
  (set `self.ThrowItemTesters` _outactors))

(event `Key|K`
  (params (Key :type "Key Structure"))
  (:`Pressed`
    (for _array_element (`self.ThrowItemTesters`)
      (if (`/Game/Item/ThrowItem/BP_ThrowItemTester.Active?` _array_element)
        (`/Game/Item/ThrowItem/BP_ThrowItemTester.ThrowTurtle` _array_element)))))

(event `Key|J`
  (params (Key :type "Key Structure"))
  (:`Pressed`
    (for _array_element (`self.ThrowItemTesters`)
      (if (`/Game/Item/ThrowItem/BP_ThrowItemTester.Active?` _array_element)
        (`/Game/Item/ThrowItem/BP_ThrowItemTester.ThrowBomb` _array_element)))))

(fn `UserConstructionScript`)