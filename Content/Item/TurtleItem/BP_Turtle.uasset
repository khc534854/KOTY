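; BP_Turtle is a launched turtle item that travels at constant horizontal speed, ricochets off obstacles and expires after a lifespan or on overlapping another turtle.
; Each Tick applies gravity, then uses a downward trace to adjust vertical velocity near the ground and keep a minimum height.
; A radial fan of horizontal traces sums reflection vectors into a new direction, with per-ray tick cooldowns preventing repeated bounces, before a swept move.
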(event `Initialize`
  (params (ShootDir :type "Vector Structure") (GravityDir :type "Vector Structure"))
  ; 초기화
  (set `self.MovingDir` ShootDir)
  (set `self.Active?` true)
  (`self.SetLifeSpan` 8.0))

(event `self.ReceiveActorBeginOverlap`
  (params (OtherActor :type "Actor Object Reference"))
  ; 충돌
  (cast `/Game/Item/TurtleItem/BP_Turtle` OtherActor)
  (`self.K2_DestroyActor`))

(event `self.ReceiveTick`
  (params (DeltaSeconds :type "Float (single-precision)"))
  (bind _returnvalue (`self.K2_GetActorLocation`))
  (bind _returnvalue_2 (`self.K2_GetActorLocation`))
  (bind (_velocity_x _velocity_y _velocity_z) (`KismetMathLibrary.BreakVector` (`self.Velocity`)))
  (bind (_surfacelocation_x _surfacelocation_y _surfacelocation_z) (`KismetMathLibrary.BreakVector` (`self.SurfaceLocation`)))
  (bind _reflections (`self.Reflections`))
  (bind (_velocity_x_2 _velocity_y_2 _velocity_z_2) (`KismetMathLibrary.BreakVector` (`self.Velocity`)))
  (bind (_velocity_x_3 _velocity_y_3) (`KismetMathLibrary.BreakVector` (`self.Velocity`)))
  (bind (_velocity_x_4 _velocity_y_4 _velocity_z_3) (`KismetMathLibrary.BreakVector` (`self.Velocity`)))
  (bind (_returnvalue_x _returnvalue_y) (`KismetMathLibrary.BreakVector` (* (`self.MovingDir`) (`self.Speed`))))
  (if (`self.Active?`)
    (`|ExecutionSequence`
      (:`then_0`
        ; 이번 이동 속도 연산
        (set `self.Velocity` (`KismetMathLibrary.MakeVector` _returnvalue_x _returnvalue_y (+ _velocity_z_2 (* (`self.GravityForce`) (`GameplayStatics.GetWorldDeltaSeconds`))))))
      (:`then_1`
        ; 바닥과의 충돌울 감지하고 튕겨내는 속도를 연산한다
        (bind (_outhit _returnvalue_3) (`KismetSystemLibrary.LineTraceSingle` _returnvalue (- _returnvalue (* 500.0 (`self.GetActorUpVector`))) "TraceTypeQuery1"))
        (if _returnvalue_3
          (bind _output_get (set `self.SurfaceLocation` (`.ImpactPoint` (`GameplayStatics.BreakHitResult` _outhit))))
          (if (< (`KismetMathLibrary.Vector_Distance` _output_get (`self.K2_GetActorLocation`)) 60.0)
            (if (>= _velocity_z_3 5.0)
              (set `self.Velocity` (`KismetMathLibrary.MakeVector` _velocity_x _velocity_y (* _velocity_z -0.8)))
              (else
                (set `self.Velocity` (`KismetMathLibrary.MakeVector` _velocity_x_3 _velocity_y_3)))))))
      (:`then_2`
        (`KismetArrayLibrary.Array_Clear` (`self.Reflections`))
        (for _index (range 15)
          (bind _returnvalue_4 (* _index 24))
          ; 360도 라인 트레이스
          (bind (_outhit_2 _returnvalue_5) (`KismetSystemLibrary.LineTraceSingle` :`Start` _returnvalue_2 :`End` (+ _returnvalue_2 (* (`KismetMathLibrary.MakeVector` (`KismetMathLibrary.DegCos` (`KismetMathLibrary.Conv_IntToDouble` _returnvalue_4)) (`KismetMathLibrary.DegSin` (`KismetMathLibrary.Conv_IntToDouble` _returnvalue_4))) 70.0)) :`TraceChannel` "TraceTypeQuery1" :`DrawTime` 0.1))
          (if _returnvalue_5
            ; 다음 5틱 동안 이 반사가 비활성화 된다
            (if (<= (`BlueprintMapLibrary.Map_Find` (`self.CollisionMap`) _index) 0)
              (`BlueprintMapLibrary.Map_Add` (`self.CollisionMap`) _index 5)
              (bind _returnvalue_6 (`KismetMathLibrary.MakeVector` (.x (`.ImpactNormal` (`GameplayStatics.BreakHitResult` _outhit_2))) (.y (`.ImpactNormal` (`GameplayStatics.BreakHitResult` _outhit_2)))))
              (`KismetArrayLibrary.Array_Add` (`self.Reflections`) (`KismetMathLibrary.Normal` (+ (`self.Velocity`) (* (`KismetMathLibrary.Dot_VectorVector` (* -1.0 (`self.Velocity`)) _returnvalue_6) _returnvalue_6 2.0)))))
            (else
              ; 충돌이 없다면 충돌 맵의 틱 카운트를 하나 낮춘다
              (`BlueprintMapLibrary.Map_Add` (`self.CollisionMap`) _index (`KismetMathLibrary.Max` (- (`BlueprintMapLibrary.Map_Find` (`self.CollisionMap`) _index) 1))))))
        ; Comment
        (set `self.Reflection` (0.0 0.0 0.0))
        (if (`KismetArrayLibrary.Array_IsNotEmpty` _reflections)
          (for _array_element _reflections
            (set `self.Reflection` (+ _array_element (`self.Reflection`))))
          ; 속도 업데이트
          (bind _output_get_2 (set `self.MovingDir` (`KismetMathLibrary.MakeVector` (.x (`KismetMathLibrary.Normal` (`self.Reflection`))) (.y (`KismetMathLibrary.Normal` (`self.Reflection`))))))
          (bind (_returnvalue_x_2 _returnvalue_y_2) (`KismetMathLibrary.BreakVector` (* _output_get_2 (`self.Speed`))))
          (set `self.Velocity` (`KismetMathLibrary.MakeVector` _returnvalue_x_2 _returnvalue_y_2))))
      (:`then_3`
        ; 속도만큼 이동하지만 바닥과의 최소 거리를 유지
        (`self.K2_SetActorLocation` (`KismetMathLibrary.MakeVector` (.x (+ (* (`self.Velocity`) (`GameplayStatics.GetWorldDeltaSeconds`)) (`self.K2_GetActorLocation`))) (.y (+ (* (`self.Velocity`) (`GameplayStatics.GetWorldDeltaSeconds`)) (`self.K2_GetActorLocation`))) (`KismetMathLibrary.FMax` (.z (+ (* (`self.Velocity`) (`GameplayStatics.GetWorldDeltaSeconds`)) (`self.K2_GetActorLocation`))) (+ _surfacelocation_z 60.0))) true)))))

(fn `UserConstructionScript`)