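; Test actor that launches BP_Turtle items from an Arrow component.
; ShootTurtle spawns a turtle at the arrow with only its yaw, then initializes it with the arrow's full forward vector and a zero gravity direction.
; When Rotate is set, Tick sweeps the arrow's world yaw side to side on a sine of accumulated time while holding a fixed pitch.
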(event `ShootTurtle`
  (bind _arrow (`self.Arrow`))
  (bind (_returnvalue_roll _returnvalue_pitch _returnvalue_yaw) (`KismetMathLibrary.BreakRotator` (`SceneComponent.K2_GetComponentRotation` _arrow)))
  (bind _returnvalue (`|SpawnActorFromClass` "/Game/Item/TurtleItem/BP_Turtle.BP_Turtle_C" (`KismetMathLibrary.MakeTransform` (`SceneComponent.K2_GetComponentLocation` _arrow) (`KismetMathLibrary.MakeRotator` 0.0 0.0 _returnvalue_yaw)) "Undefined" "MultiplyWithRoot" null null))
  (`/Game/Item/TurtleItem/BP_Turtle.Initialize` _returnvalue (`SceneComponent.GetForwardVector` (`self.Arrow`)) (0.0 0.0 0.0)))

(event `self.ReceiveTick`
  (params (DeltaSeconds :type "Float (single-precision)"))
  (if (`self.Rotate?`)
    (bind _output_get (set `self.ElapsedTime` (+ DeltaSeconds (`self.ElapsedTime`))))
    (`SceneComponent.K2_SetWorldRotation` (`self.Arrow`) (`KismetMathLibrary.MakeRotator` 0.0 45.0 (* (`KismetMathLibrary.Sin` _output_get) 45.0)) false false)))

(fn `UserConstructionScript`)