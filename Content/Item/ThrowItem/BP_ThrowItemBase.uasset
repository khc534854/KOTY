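; Base actor for throwable items, moved by a KotyMovement component.
; Throw scales the input direction into a velocity and starts a simulated throw with downward gravity, linear drag, step-up limit and surface bounce.
; Tick only visualizes debug data: line traces along velocity and gravity, plus printed speed.
; The item destroys itself when it overlaps another throw item.
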(event `self.ReceiveActorBeginOverlap`
  (params (OtherActor :type "Actor Object Reference"))
  (cast `/Game/Item/ThrowItem/BP_ThrowItemBase` OtherActor)
  (`self.K2_DestroyActor`))

(event `self.ReceiveTick`
  (params (DeltaSeconds :type "Float (single-precision)"))
  (bind _returnvalue (+ (`self.K2_GetActorLocation`) (* (`KismetMathLibrary.Normal` (`KotyMovementComponent.MoveVelocity` (`self.KotyMovement`))) 50.0)))
  (`KismetSystemLibrary.LineTraceSingle` :`Start` (`self.K2_GetActorLocation`) :`End` (+ (`self.K2_GetActorLocation`) (`KotyMovementComponent.MoveVelocity` (`self.KotyMovement`))) :`TraceChannel` "TraceTypeQuery1" :`DrawDebugType` "ForDuration" :`DrawTime` 0.1)
  (`KismetSystemLibrary.PrintString` (`KismetStringLibrary.Conv_DoubleToString` (`KismetMathLibrary.VSize` (`KotyMovementComponent.MoveVelocity` (`self.KotyMovement`)))) true true (struct :`G` 0.66 :`B` 1.0 :`A` 1.0) 1.0)
  (`KismetSystemLibrary.LineTraceSingle` :`Start` _returnvalue :`End` (+ _returnvalue (* 1000.0 (`KotyMovementComponent.GravityDir` (`self.KotyMovement`)))) :`TraceChannel` "TraceTypeQuery1" :`DrawDebugType` "ForDuration" :`TraceColor` (struct :`B` 1.0 :`A` 1.0) :`DrawTime` 0.1))

(fn `Throw`
  (params (InMoveDir :type "Vector Structure"))
  (`KotyMovementComponent.ThrowLinearDrag` (`self.KotyMovement`) true (`KismetMathLibrary.Vector_Down`) 3000.0 0.1 3.0 (* InMoveDir 1000.0) 0.25))

(fn `UserConstructionScript`)