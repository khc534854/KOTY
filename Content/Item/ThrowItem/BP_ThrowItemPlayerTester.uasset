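; Test actor that launches player throwable items, a green turtle or a black bomb, from its Arrow component.
; ThrowTurtle and ThrowBomb spawn the item and call Throw with the arrow's forward vector and the player kart's gravity direction.
; Each throw then sets a short life span on the tester itself.
; When Rotate is on, Tick swings the arrow's yaw on a sine wave at a fixed upward pitch.
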(event `ThrowTurtle`
  ; Comment
  (bind _returnvalue (`|SpawnActorFromClass` "/Game/Item/ThrowItem/BP_GreenTurtlePlayerItem.BP_GreenTurtlePlayerItem_C" (`SceneComponent.K2_GetComponentToWorld` (`self.Arrow`)) "Undefined" "MultiplyWithRoot" null null))
  (bind _asbp_throw_item_player_base (cast `/Game/Item/ThrowItem/BP_ThrowItemPlayerBase` _returnvalue))
  (bind _asbpc_player_kart (cast `/Game/Koty/PlayerKart/BPC_PlayerKart` (`GameplayStatics.GetPlayerPawn` 0)))
  (`/Game/Item/ThrowItem/BP_ThrowItemPlayerBase.Throw` _asbp_throw_item_player_base (`SceneComponent.GetForwardVector` (`self.Arrow`)) (`C_KartBase.GravityDirection` _asbpc_player_kart))
  (`self.SetLifeSpan` 10.0))

(event `ThrowBomb`
  ; Comment
  (bind _returnvalue (`|SpawnActorFromClass` "/Game/Item/ThrowItem/BP_BlackBombItem1.BP_BlackBombItem1_C" (`SceneComponent.K2_GetComponentToWorld` (`self.Arrow`)) "Undefined" "MultiplyWithRoot" null null))
  (bind _asbp_throw_item_player_base (cast `/Game/Item/ThrowItem/BP_ThrowItemPlayerBase` _returnvalue))
  (bind _asbpc_player_kart (cast `/Game/Koty/PlayerKart/BPC_PlayerKart` (`GameplayStatics.GetPlayerPawn` 0)))
  (`/Game/Item/ThrowItem/BP_ThrowItemPlayerBase.Throw` _asbp_throw_item_player_base (`SceneComponent.GetForwardVector` (`self.Arrow`)) (`C_KartBase.GravityDirection` _asbpc_player_kart))
  (`self.SetLifeSpan` 10.0))

(event `self.ReceiveTick`
  (params (DeltaSeconds :type "Float (single-precision)"))
  (if (`self.Rotate?`)
    (bind _output_get (set `self.ElapsedTime` (+ DeltaSeconds (`self.ElapsedTime`))))
    (`SceneComponent.K2_SetWorldRotation` (`self.Arrow`) (`KismetMathLibrary.MakeRotator` 0.0 45.0 (* (`KismetMathLibrary.Sin` _output_get) 45.0)) false false)))

(fn `UserConstructionScript`)