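; Test actor that spawns and throws green turtle and black bomb items from its Arrow component.
; ThrowTurtle and ThrowBomb each spawn their item at the arrow's transform, call the BP_ThrowItemBase Throw along its forward vector and give it a short lifespan.
; When Rotate is set, Tick swings the arrow's yaw side to side with a sine wave at fixed pitch, varying the throw direction.
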(event `ThrowTurtle`
  ; Comment
  (bind _returnvalue (`|SpawnActorFromClass` "/Game/Item/ThrowItem/BP_GreenTurtleItem.BP_GreenTurtleItem_C" (`SceneComponent.K2_GetComponentToWorld` (`self.Arrow`)) "Undefined" "MultiplyWithRoot" null null))
  (bind _asbp_throw_item_base (cast `/Game/Item/ThrowItem/BP_ThrowItemBase` _returnvalue))
  (`/Game/Item/ThrowItem/BP_ThrowItemBase.Throw` _asbp_throw_item_base (`SceneComponent.GetForwardVector` (`self.Arrow`)))
  (`self.SetLifeSpan` _asbp_throw_item_base 8.0))

(event `ThrowBomb`
  ; Comment
  (bind _returnvalue (`|SpawnActorFromClass` "/Game/Item/ThrowItem/BP_BlackBombItem.BP_BlackBombItem_C" (`SceneComponent.K2_GetComponentToWorld` (`self.Arrow`)) "Undefined" "MultiplyWithRoot" null null))
  (bind _asbp_throw_item_base (cast `/Game/Item/ThrowItem/BP_ThrowItemBase` _returnvalue))
  (`/Game/Item/ThrowItem/BP_ThrowItemBase.Throw` _asbp_throw_item_base (`SceneComponent.GetForwardVector` (`self.Arrow`)))
  (`self.SetLifeSpan` _asbp_throw_item_base 8.0))

(event `self.ReceiveTick`
  (params (DeltaSeconds :type "Float (single-precision)"))
  (if (`self.Rotate?`)
    (bind _output_get (set `self.ElapsedTime` (+ DeltaSeconds (`self.ElapsedTime`))))
    (`SceneComponent.K2_SetWorldRotation` (`self.Arrow`) (`KismetMathLibrary.MakeRotator` 0.0 45.0 (* (`KismetMathLibrary.Sin` _output_get) 45.0)) false false)))

(fn `UserConstructionScript`)