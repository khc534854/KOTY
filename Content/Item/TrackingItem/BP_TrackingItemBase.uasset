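; Base actor for tracking items that steer themselves toward a target through a KotyMovement component.
; Each Tick it slerps velocity toward the Target, set via SetTarget, when that actor is within DetectLength.
; Otherwise, in one TrackingMode, it follows the first guide spline from BP_ItemTestGameMode, heading to its closest point when far and along its direction when near.
; MoveAlongTrackingGuide is empty, and the construction script's line trace result is unused.
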(event `self.ReceiveBeginPlay`
  (bind _asbp_item_test_game_mode (cast `/Game/Item/Default/BP_ItemTestGameMode` (`GameplayStatics.GetGameMode`)))
  (set `self.ItemTestGameMode` _asbp_item_test_game_mode))

(event `self.ReceiveTick`
  (params (DeltaSeconds :type "Float (single-precision)"))
  (bind _trackingguidesplines (`/Game/Item/Default/BP_ItemTestGameMode.TrackingGuideSplines` (`self.ItemTestGameMode`)))
  (bind _returnvalue (+ (`self.K2_GetActorLocation`) (`KismetMathLibrary.Normal` (`KotyMovementComponent.MoveVelocity` (`self.KotyMovement`)))))
  (bind _spline (`/Game/Item/TrackingItem/BP_TrackingGuideOnGround.Spline` (`|GetArrayItem` _trackingguidesplines)))
  (bind _returnvalue_2 (- (`SplineComponent.FindLocationClosestToWorldLocation` _spline _returnvalue "World") (`self.K2_GetActorLocation`)))
  (`/Engine/EditorBlueprintResources/StandardMacros.IsValid` (`self.Target`)
    (:`Is Valid`
      ; Comment
      (if (< (`KismetMathLibrary.VSize` (- (`self.K2_GetActorLocation` (`self.Target`)) (`self.K2_GetActorLocation`))) (`self.DetectLength`))
        (`KotyMovementComponent.SLerpVelocity` (`self.KotyMovement`) (`KismetMathLibrary.Normal` (- (`self.K2_GetActorLocation` (`self.Target`)) (`self.K2_GetActorLocation`))))
        (else
          ; Comment
          (if (`|EnumEquality` (`self.TrackingMode`) "NewEnumerator3") :!label _label
            ; Comment
            (if (`KismetArrayLibrary.Array_IsNotEmpty` _trackingguidesplines)
              (if (< (`KismetMathLibrary.VSize` _returnvalue_2) 300.0)
                (`KotyMovementComponent.SLerpVelocity` (`self.KotyMovement`) (`SplineComponent.FindDirectionClosestToWorldLocation` _spline _returnvalue "World"))
                (else
                  (`KotyMovementComponent.SLerpVelocity` (`self.KotyMovement`) (`KismetMathLibrary.Normal` _returnvalue_2)))))))))
    (:`Is Not Valid`
      (goto _label))))

(fn `MoveAlongTrackingGuide`)

(fn `SetTarget`
  (params (TargetActor :type "Actor Object Reference"))
  (set `self.Target` TargetActor))

(fn `UserConstructionScript`
  (`KismetSystemLibrary.LineTraceSingle` (`self.K2_GetActorLocation`) (0.0 0.0 0.0) "TraceTypeQuery1"))