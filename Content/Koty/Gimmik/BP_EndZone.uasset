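; BP_EndZone is a finish-line trigger that counts laps for player karts.
; On Box overlap, it increments a BPC_PlayerKart's CurrentLaps only if MaxProgressPointIndex has passed a threshold, guarding against uncompleted laps.
; It then branches on the lap count, resetting the progress index above the limit and otherwise calling FinishLaps through a DoOnce.
; The DoOnce is never reset, so each zone instance makes that call only once.
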(event `self.Box.OnComponentBeginOverlap`
  (params (OverlappedComponent :type "PrimitiveComponent Object Reference") (OtherActor :type "Actor Object Reference") (OtherComp :type "PrimitiveComponent Object Reference") (OtherBodyIndex :type Integer) (bFromSweep :type Boolean) (SweepResult :type "HitResult Structure (by ref)"))
  (bind _asbpc_player_kart (cast `/Game/Koty/PlayerKart/BPC_PlayerKart` OtherActor))
  (if (and true (> (`C_PlayerKart.MaxProgressPointIndex` _asbpc_player_kart) 10))
    (bind _currentlaps (`/Game/Koty/PlayerKart/BPC_PlayerKart.CurrentLaps` _asbpc_player_kart))
    (`/Engine/EditorBlueprintResources/StandardMacros.IncrementInt` _currentlaps
      (:`  `
        (if (> _currentlaps 2)
          (set `C_PlayerKart.MaxProgressPointIndex` 0 _asbpc_player_kart)
          (else
            (`/Engine/EditorBlueprintResources/StandardMacros.DoOnce` false
              (:`Completed`
                (`/Game/Koty/PlayerKart/BPC_PlayerKart.FinishLaps` _asbpc_player_kart)))))))))

(fn `UserConstructionScript`)