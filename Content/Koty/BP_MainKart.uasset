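; Player kart Blueprint with hand-coded movement, driven by Enhanced Input for throttle and steering.
; Held throttle builds an acceleration timer that decays on release and is cubed into a capped speed, while steering adds clamped yaw.
; Each tick a short downward trace snaps the kart to ground; without a hit, forward speed plus gravity updates the velocity vector.
; That vector is recomputed only when airborne but moves the kart every tick.
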(event `self.ReceiveBeginPlay`
  (bind _returnvalue (`GameplayStatics.GetPlayerController` 0))
  (`/Engine/EditorBlueprintResources/StandardMacros.IsValid` _returnvalue
    (:`Is Valid`
      (`EnhancedInputSubsystemInterface.AddMappingContext` (pcsubsystem `EnhancedInputLocalPlayerSubsystem` _returnvalue) "/Game/Koty/Input/IMC_Player.IMC_Player" 0 (struct)))))

(event `self.ReceiveTick`
  (params (DeltaSeconds :type "Float (single-precision)"))
  (bind _returnvalue (`self.K2_GetActorLocation`))
  (if (not (`self.bIsAcceleration`))
    (set `self.AccelerationTime` (`KismetMathLibrary.FClamp` (- (`self.AccelerationTime`) (`GameplayStatics.GetWorldDeltaSeconds`)) 0.0 (`self.MaxTime`))))
  (`self.SetSpeed`)
  (bind (_outhit _returnvalue_2) (`KismetSystemLibrary.LineTraceSingle` :`Start` _returnvalue :`End` (+ _returnvalue (0.0 0.0 -50.0)) :`TraceChannel` "TraceTypeQuery1" :`DrawDebugType` "ForDuration"))
  (if _returnvalue_2
    (bind (_bblockinghit _binitialoverlap _time _distance _location) (`GameplayStatics.BreakHitResult` _outhit))
    (`self.K2_SetActorLocation` (`KismetMathLibrary.MakeVector` (.x _location) (.y _location) (+ (.z _location) 50.0)))
    (else
      (`self.K2_SetActorLocation` (+ (`self.K2_GetActorLocation`) (* (`self.SetAcceleration`) (`GameplayStatics.GetWorldDeltaSeconds`))))))
  (`self.K2_SetActorLocation` (+ (* (`GameplayStatics.GetWorldDeltaSeconds`) (`self.CurrentDirectionwithSpeed`)) (`self.K2_GetActorLocation`))))

(event `EnhancedInput|/Game/Koty/Input/IA_Accelerator`
  (params (ActionValue :type "Float (double-precision)") (ElapsedSeconds :type "Float (double-precision)") (TriggeredSeconds :type "Float (double-precision)") (InputAction :type "InputAction Object Reference" :default "/Game/Koty/Input/IA_Accelerator.IA_Accelerator"))
  (:`Triggered`
    (set `self.AccelerationTime` (+ (* (`self.AccelerationTime`) ActionValue) (`GameplayStatics.GetWorldDeltaSeconds`)))
    (set `self.bIsAcceleration` true))
  (:`Completed`
    (set `self.bIsAcceleration` false)))

(event `EnhancedInput|/Game/Koty/Input/IA_Handling`
  (params (ActionValue :type "Float (double-precision)") (ElapsedSeconds :type "Float (double-precision)") (TriggeredSeconds :type "Float (double-precision)") (InputAction :type "InputAction Object Reference" :default "/Game/Koty/Input/IA_Handling.IA_Handling"))
  (:`Triggered`
    (`self.Turn` ActionValue ElapsedSeconds)))

(fn `Move`
  (params (`X Axis` :type "Float (double-precision)"))
  (`self.K2_SetActorLocation` (+ (* (`self.GetActorForwardVector`) (`GameplayStatics.GetWorldDeltaSeconds`) (* `X Axis` (`self.CurrnetSpeed`))) (`self.K2_GetActorLocation`))))

(fn `SetAcceleration`
  (returns (Output_Get :type "Vector Structure"))
  (bind _currnetspeed (`self.CurrnetSpeed`))
  (bind _output_get (set `self.CurrentDirectionwithSpeed` (`KismetMathLibrary.ClampVectorSize` (+ (* (`self.GetActorForwardVector`) _currnetspeed) (`KismetMathLibrary.MakeVector` 0.0 0.0 (* (`self.GravityValue`) -1.0))) 0.0 _currnetspeed)))
  (return _output_get))

(fn `SetSpeed`
  (bind _returnvalue (* (`KismetMathLibrary.MultiplyMultiply_FloatFloat` (`self.AccelerationTime`) 3.0) (`self.AcceleratorValue`)))
  (if (>= _returnvalue (`self.MaxSpeed`))
    (set `self.MaxTime` (`self.AccelerationTime`)))
  (set `self.CurrnetSpeed` (`KismetMathLibrary.FClamp` _returnvalue 0.0 (`self.MaxSpeed`))))

(fn `Turn`
  (params (`New Rotation Z (Yaw)` :type "Float (single-precision)") (B :type "Float (double-precision)"))
  (bind (_returnvalue_roll _returnvalue_pitch _returnvalue_yaw) (`KismetMathLibrary.BreakRotator` (`self.K2_GetActorRotation`)))
  (`self.K2_SetActorRotation` (`KismetMathLibrary.MakeRotator` _returnvalue_roll _returnvalue_pitch (+ _returnvalue_yaw (`KismetMathLibrary.FClamp` (* `New Rotation Z (Yaw)` B (`self.HandlingValue`)) -10.0 10.0)))))

(fn `UserConstructionScript`)