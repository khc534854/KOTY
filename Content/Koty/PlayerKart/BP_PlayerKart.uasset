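; Player kart pawn driven by Enhanced Input for throttle, steering and drift, moved kinematically without physics or sweeps.
; Throttle builds an acceleration timer whose cube sets speed; coasting decays it on flat ground or shifts it downhill via Front/Back height.
; Each Tick a downward trace snaps the kart to ground and its normal, otherwise applies constant fall and pitches toward travel.
; Drift turns also combine in Front's relative rotation.
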(event `self.ReceiveBeginPlay`
  (bind _returnvalue (`GameplayStatics.GetPlayerController` 0))
  (`/Engine/EditorBlueprintResources/StandardMacros.IsValid` _returnvalue
    (:`Is Valid`
      (`EnhancedInputSubsystemInterface.AddMappingContext` (pcsubsystem `EnhancedInputLocalPlayerSubsystem` _returnvalue) "/Game/Koty/PlayerKart/Input/IMC_Player.IMC_Player" 0 (struct))
      (set `self.MaxTime` (`KismetMathLibrary.MultiplyMultiply_FloatFloat` (/ (`self.MaxSpeed`) (`self.AcceleratorValue`)) 0.333)))))

(event `self.ReceiveTick`
  (params (DeltaSeconds :type "Float (single-precision)"))
  (bind _returnvalue (`self.K2_GetActorLocation`))
  (if (not (`self.bIsAcceleration`))
    (`self.DecreaseAccelTime`))
  (`self.SetSpeed`)
  (bind (_outhit _returnvalue_2) (`KismetSystemLibrary.LineTraceSingle` :`Start` _returnvalue :`End` (+ _returnvalue (0.0 0.0 -50.0)) :`TraceChannel` "TraceTypeQuery1" :`DrawDebugType` "ForDuration"))
  (if _returnvalue_2
    (bind (_bblockinghit _binitialoverlap _time _distance _location _impactpoint _normal _impactnormal) (`GameplayStatics.BreakHitResult` _outhit))
    (`self.K2_SetActorRotation` (`KismetMathLibrary.MakeRotFromZX` _impactnormal (`self.GetActorForwardVector`)))
    (`self.K2_SetActorLocation` (+ _location (`self.SetGroundDirection`) (0.0 0.0 49.0)))
    (set `self.bIsGround` true)
    (else
      (`self.K2_SetActorLocation` (+ (`self.K2_GetActorLocation`) (`self.SetAirDirection`)))
      (set `self.bIsGround` false))))

(event `EnhancedInput|/Game/Koty/PlayerKart/Input/IA_Accelerator`
  (params (ActionValue :type "Float (double-precision)") (ElapsedSeconds :type "Float (double-precision)") (TriggeredSeconds :type "Float (double-precision)") (InputAction :type "InputAction Object Reference" :default "/Game/Koty/PlayerKart/Input/IA_Accelerator.IA_Accelerator"))
  (:`Triggered`
    (if (`self.bIsGround`)
      (`self.IncreaseAccelTime` ActionValue)
      (set `self.bIsAcceleration` true)))
  (:`Completed`
    (set `self.bIsAcceleration` false)))

(event `EnhancedInput|/Game/Koty/PlayerKart/Input/IA_Handling`
  (params (ActionValue :type "Float (double-precision)") (ElapsedSeconds :type "Float (double-precision)") (TriggeredSeconds :type "Float (double-precision)") (InputAction :type "InputAction Object Reference" :default "/Game/Koty/PlayerKart/Input/IA_Handling.IA_Handling"))
  (:`Triggered`
    (`self.Turn` ActionValue ElapsedSeconds)))

(event `EnhancedInput|/Game/Koty/PlayerKart/Input/IA_Drift`
  (params (ActionValue :type Boolean) (ElapsedSeconds :type "Float (double-precision)") (TriggeredSeconds :type "Float (double-precision)") (InputAction :type "InputAction Object Reference" :default "/Game/Koty/PlayerKart/Input/IA_Drift.IA_Drift"))
  (:`Triggered`
    (set `self.bISDrift` ActionValue))
  (:`Completed`
    (set `self.bISDrift` false)))

(fn `DecreaseAccelTime`
  (bind _accelerationtime (`self.AccelerationTime`))
  (bind _accelerationtime_2 (`self.AccelerationTime`))
  (bind (_returnvalue_x _returnvalue_y _returnvalue_z) (`KismetMathLibrary.BreakVector` (`SceneComponent.K2_GetComponentLocation` (`self.Front`))))
  (bind (_returnvalue_x_2 _returnvalue_y_2 _returnvalue_z_2) (`KismetMathLibrary.BreakVector` (`SceneComponent.K2_GetComponentLocation` (`self.Back`))))
  (bind _returnvalue (* (`GameplayStatics.GetWorldDeltaSeconds`) (`self.BrakeValue`)))
  (bind _returnvalue_2 (* 2.0 (`GameplayStatics.GetWorldDeltaSeconds`)))
  (if (`self.bIsGround`)
    (if (== _returnvalue_z _returnvalue_z_2)
      (if (> (`self.AccelerationTime`) 0.0)
        (set `self.AccelerationTime` (`KismetMathLibrary.FClamp` (- _accelerationtime _returnvalue) 0.0 (`self.MaxTime`)))
        (else
          (set `self.AccelerationTime` (`KismetMathLibrary.FClamp` (+ _accelerationtime _returnvalue) (* (`self.MaxTime`) -1.0) 0.0))))
      (else
        ; 경사도 체크
        (if (> _returnvalue_z _returnvalue_z_2)
          (set `self.AccelerationTime` (- _accelerationtime_2 _returnvalue_2))
          (else
            (set `self.AccelerationTime` (+ _accelerationtime_2 _returnvalue_2))))))))

(fn `IncreaseAccelTime`
  (params (A :type "Float (double-precision)"))
  (bind _returnvalue (`GameplayStatics.GetWorldDeltaSeconds`))
  (bind _maxtime (`self.MaxTime`))
  (if (> A 0.0)
    (set `self.AccelerationTime` (+ (`self.AccelerationTime`) _returnvalue))
    (else
      (set `self.AccelerationTime` (+ (`self.AccelerationTime`) (* _returnvalue -1.0)))))
  (set `self.AccelerationTime` (`KismetMathLibrary.FClamp` (`self.AccelerationTime`) (* _maxtime -1.0) _maxtime)))

(fn `Move`
  (params (`X Axis` :type "Float (double-precision)"))
  (`self.K2_SetActorLocation` (+ (* (`self.GetActorForwardVector`) (`GameplayStatics.GetWorldDeltaSeconds`) (* `X Axis` (`self.CurrnetSpeed`))) (`self.K2_GetActorLocation`))))

(fn `SetAirDirection`
  (returns (direction :type "Vector Structure"))
  (bind _returnvalue (`self.K2_GetActorLocation`))
  (bind _returnvalue_2 (+ (* (`self.GetActorForwardVector`) (`self.CurrnetSpeed`)) (`KismetMathLibrary.MakeVector` 0.0 0.0 (* (`self.GravityValue`) -1.0))))
  (bind (_returnvalue_roll _returnvalue_pitch _returnvalue_yaw) (`KismetMathLibrary.BreakRotator` (`KismetMathLibrary.FindLookAtRotation` _returnvalue (+ _returnvalue_2 _returnvalue))))
  (bind _output_get (set `self.Direction` _returnvalue_2))
  (`self.K2_SetActorRotation` (`KismetMathLibrary.MakeRotator` _returnvalue_roll (`KismetMathLibrary.FClamp` _returnvalue_pitch -20.0 50.0) _returnvalue_yaw))
  (return _output_get))

(fn `SetGroundDirection`
  (returns (direction :type "Vector Structure"))
  (bind _output_get (set `self.Direction` (* (`self.GetActorForwardVector`) (`self.CurrnetSpeed`))))
  (return _output_get))

(fn `SetSpeed`
  (bind _maxspeed (`self.MaxSpeed`))
  (set `self.CurrnetSpeed` (`KismetMathLibrary.FClamp` (* (`KismetMathLibrary.MultiplyMultiply_FloatFloat` (`self.AccelerationTime`) 3.0) (`self.AcceleratorValue`)) (* _maxspeed -1.0) _maxspeed)))

(fn `Turn`
  (params (`New Rotation Z (Yaw)` :type "Float (single-precision)") (B :type "Float (double-precision)"))
  (bind (_returnvalue_roll _returnvalue_pitch _returnvalue_yaw) (`KismetMathLibrary.BreakRotator` (`self.K2_GetActorRotation`)))
  (bind (_returnvalue_roll_2 _returnvalue_pitch_2 _returnvalue_yaw_2) (`KismetMathLibrary.BreakRotator` (`self.K2_GetActorRotation`)))
  (bind _returnvalue (`KismetMathLibrary.FClamp` (* `New Rotation Z (Yaw)` B (`self.HandlingValue`)) -10.0 10.0))
  (if (`self.bISDrift`)
    (`self.K2_SetActorRotation` (`KismetMathLibrary.ComposeRotators` (`SceneComponent.RelativeRotation` (`self.Front`)) (`KismetMathLibrary.MakeRotator` _returnvalue_roll_2 _returnvalue_pitch_2 (+ _returnvalue_yaw_2 _returnvalue))))
    (else
      (`self.K2_SetActorRotation` (`KismetMathLibrary.MakeRotator` _returnvalue_roll _returnvalue_pitch (+ _returnvalue_yaw _returnvalue))))))

(fn `UserConstructionScript`)