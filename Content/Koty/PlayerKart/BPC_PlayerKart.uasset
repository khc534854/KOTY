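; Player kart Blueprint that triggers test turtle throws from item input.
; On BeginPlay it caches all BP_ThrowItemPlayerTester actors in the level, then calls ThrowTurtle on each when IA_Item completes.
; Afterburner exhaust spawning for high AddSpeed and a bomb throw are present but unconnected, and Tick and the construction script are empty.
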(event `self.ReceiveBeginPlay`
  (bind _outactors (`GameplayStatics.GetAllActorsOfClass` "/Game/Item/ThrowItem/BP_ThrowItemPlayerTester.BP_ThrowItemPlayerTester_C"))
  (set `self.ThrowItemTesters_0` _outactors))

(event `EnhancedInput|/Game/Koty/PlayerKart/Input/IA_Item`
  (params (ActionValue :type Boolean) (ElapsedSeconds :type "Float (double-precision)") (TriggeredSeconds :type "Float (double-precision)") (InputAction :type "InputAction Object Reference" :default "/Game/Koty/PlayerKart/Input/IA_Item.IA_Item"))
  (:`Completed`
    (for _array_element (`self.ThrowItemTesters_0`)
      (if true
        (`/Game/Item/ThrowItem/BP_ThrowItemPlayerTester.ThrowTurtle` _array_element)))))

(event `self.ReceiveTick`
  (params (DeltaSeconds :type "Float (single-precision)")))

(fn `UserConstructionScript`)